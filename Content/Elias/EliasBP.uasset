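; Elias is an AI-moved character Blueprint that acts out beats as lines start, either walking or gesturing.
; OnLineStarted stops the last montage, then either sends a Walk beat's MovePoint to MoveElias or plays and stores a Gesture beat's montage.
; MoveElias uses AI MoveTo and matches the target actor's rotation on arrival, with a default controller spawned at BeginPlay if missing.
; IsWalking reports horizontal movement, while FacePlayer is an empty stub.
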(event `self.ReceiveBeginPlay`
  (set `CharacterMovementComponent.MaxWalkSpeed` 100.0 (`self.CharacterMovement`))
  (`/Engine/EditorBlueprintResources/StandardMacros.IsValid` (`self.GetController`)
    (:`Is Not Valid`
      (`self.SpawnDefaultController`))))

(event `MoveElias`
  (params (Location :type "TargetPoint Object Reference"))
  (`|AIMoveTo` self (0.0 0.0 0.0) Location 20.0
    (:`OnSuccess`
      (`self.K2_SetActorRotation` (`self.K2_GetActorRotation` Location)))))

(fn `FacePlayer`)

(fn `IsWalking`
  (returns (IsWaklking :type Boolean))
  (return (> (`KismetMathLibrary.VSizeXY` (`MovementComponent.Velocity` (`self.CharacterMovement`))) 5.0)))

(fn `OnLineStarted`
  (params (BeatInfo :type "/Game/Ending/BeatsStruct Structure"))
  (bind (_action _movepoint _animation) (break `/Game/Ending/BeatsStruct` BeatInfo))
  (`self.StopAnimMontage` (`self.LastAnimMonatge`))
  (switch `/Game/Ending/ActionTypes` _action
    (:`NewEnumerator1`
      (`self.MoveElias` _movepoint))
    (:`NewEnumerator2`
      (bind _output_get (set `self.LastAnimMonatge` _animation))
      (`self.PlayAnimMontage` _output_get))))

(fn `UserConstructionScript`)